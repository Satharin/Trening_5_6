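; Firefly actor that flies in an endless loop through the BP_CornerActor actors placed in the level.
; BeginPlay gathers the corners in GetAllActorsOfClass order, with no sorting, and targets the one at CurrentIndex.
; Each Tick, MoveFireflyToCorner steps a Speed-scaled fraction of the remaining offset, so it slows on approach.
; Within a small radius of the target it advances to the next corner, wrapping to the first.
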(event `self.ReceiveBeginPlay`
  (bind _outactors (`GameplayStatics.GetAllActorsOfClass` "/Game/Blueprints/BP_CornerActor.BP_CornerActor_C"))
  (bind _output_get (set `self.Corners` _outactors))
  (set `self.TargetLocation` (`self.K2_GetActorLocation` (`|GetArrayItem` _output_get (`self.CurrentIndex`)))))

(event `self.ReceiveTick`
  (params (DeltaSeconds :type "Float (single-precision)"))
  (bind _returnvalue (`self.MoveFireflyToCorner` DeltaSeconds))
  (`self.K2_SetActorLocation` _returnvalue)
  (if (and (< (`KismetMathLibrary.Vector_Distance` (`self.K2_GetActorLocation`) (`self.TargetLocation`)) 100.0) (`self.CanSwitchTarget`))
    (set `self.CanSwitchTarget` false)
    (bind _result (`/Engine/EditorBlueprintResources/StandardMacros.IncrementInt` (`self.CurrentIndex`))
      (:`  `
        (set `self.CurrentIndex` _result)
        (if (>= (`self.CurrentIndex`) (`KismetArrayLibrary.Array_Length` (`self.Corners`)))
          (set `self.CurrentIndex` 0)
          (set `self.TargetLocation` (`self.K2_GetActorLocation` (`|GetArrayItem` (`self.Corners`) (`self.CurrentIndex`))))
          (set `self.CanSwitchTarget` true)
          (else
            (set `self.TargetLocation` (`self.K2_GetActorLocation` (`|GetArrayItem` (`self.Corners`) (`self.CurrentIndex`))))
            (set `self.CanSwitchTarget` true)))))))

(fn `MoveFireflyToCorner`
  (params (DeltaSeconds :type "Float (double-precision)"))
  (returns (ReturnValue :type "Vector Structure"))
  (locals (VectorLength :type "Float (double-precision)" :default 0.0))
  (return (+ (`self.K2_GetActorLocation`) (* (- (`self.TargetLocation`) (`self.K2_GetActorLocation`)) (* (`self.Speed`) DeltaSeconds)))))

(fn `UserConstructionScript`)