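; BP_Tree is a tree actor with a firefly mesh that orbits and bobs, and hides when a pawn comes near.
; Tick yaws the firefly's scene pivot by delta time squared, making rotation frame-rate dependent, and drives a sine wave for its height.
; A volume overlap by any pawn plays a scale timeline to hide the firefly, reversing it on exit.
; A separate WinkIn event scales it into existence with another timeline.
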(event `self.TreeFireflyVolume.OnComponentBeginOverlap`
  (params (OverlappedComponent :type "PrimitiveComponent Object Reference") (OtherActor :type "Actor Object Reference") (OtherComp :type "PrimitiveComponent Object Reference") (OtherBodyIndex :type Integer) (bFromSweep :type Boolean) (SweepResult :type "HitResult Structure (by ref)"))
  ;[1 0.01777 0] Hide and Unhide TreeFirefly
  (cast `Pawn` OtherActor)
  (bind (_direction _scale) (`Timeline|HideTreeFirefly` :!via `PlayFromStart` :!label _label)
    (:`Update`
      (`self.ScaleTreeFirefly` _scale))))

(event `self.TreeFireflyVolume.OnComponentEndOverlap`
  (params (OverlappedComponent :type "PrimitiveComponent Object Reference") (OtherActor :type "Actor Object Reference") (OtherComp :type "PrimitiveComponent Object Reference") (OtherBodyIndex :type Integer))
  ;[1 0.01777 0] Hide and Unhide TreeFirefly
  (cast `Pawn` OtherActor)
  (goto _label :!via `ReverseFromEnd`))

(event `WinkIn`
  ;[0.5885 0.02759 0.000104 0.5] Wink Into Existence
  (bind (_direction _scalein) (`Timeline|Timeline_0`)
    (:`Update`
      (`SceneComponent.SetWorldScale3D` (`self.TreeFirelyMesh`) (`KismetMathLibrary.Conv_DoubleToVector` _scalein)))))

(event `self.ReceiveTick`
  (params (DeltaSeconds :type "Float (single-precision)"))
  (`self.FireflySpeed` DeltaSeconds)
  (`self.FireflyHeight` (`GameplayStatics.GetWorldDeltaSeconds`)))

(fn `FireflyHeight`
  (params (Height :type "Float (double-precision)"))
  (bind _returnvalue (`SceneComponent.GetRelativeTransform` (`self.TreeFirelyMesh`)))
  ; Sinusoidal Flight between -100 and 100
  (bind _output_get (set `self.Time` (+ (`self.Time`) Height)))
  (`SceneComponent.K2_SetRelativeLocation` (`self.TreeFirelyMesh`) (`KismetMathLibrary.MakeVector` (.x (.location _returnvalue)) (.y (.location _returnvalue)) (* (`KismetMathLibrary.Sin` (* _output_get 2.0)) 100.0)) false false))

(fn `FireflySpeed`
  (params (Speed :type "Float (double-precision)"))
  (`SceneComponent.K2_AddLocalRotation` (`self.TreeFireflyScene`) (`KismetMathLibrary.MakeRotator` 0.0 0.0 (* (`self.Speed`) Speed)) false false))

(fn `ScaleTreeFirefly`
  (params (Scale :type "Float (double-precision)"))
  (`SceneComponent.SetWorldScale3D` (`self.TreeFirelyMesh`) (`KismetMathLibrary.MakeVector` Scale Scale Scale)))

(fn `UserConstructionScript`)