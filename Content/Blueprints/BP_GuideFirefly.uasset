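; BP_GuideFirefly is a guide actor that leads the player along a series of BP_GuideActor points.
; On BeginPlay it gathers those actors in the order returned, with no sorting, and targets the one at the current index.
; Each tick it either moves toward its target at constant speed or waits for the player to come close.
; On arrival it stops, advances the index and prints the new target, going idle after the last point.
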(event `self.ReceiveBeginPlay`
  (bind _outactors (`GameplayStatics.GetAllActorsOfClass` "/Game/Blueprints/BP_GuideActor.BP_GuideActor_C"))
  (bind _output_get (set `self.GuidePoints` _outactors))
  (set `self.TargetLocation` (`self.K2_GetActorLocation` (`|GetArrayItem` _output_get (`self.CurrentIndex`)))))

(event `self.ReceiveTick`
  (params (DeltaSeconds :type "Float (single-precision)"))
  (if (`self.FinalLocation`)
    _
    (elif (`self.IsMoving`)
      (`self.MoveToNextTarget`)
      (if (< (`KismetMathLibrary.Vector_Distance` (`self.K2_GetActorLocation`) (`self.TargetLocation`)) 10.0)
        (set `self.IsMoving` false)
        (`self.ChangeIndexAndTarget`))
      (else
        (`self.ChangeToMoving`)))))

(fn `ChangeIndexAndTarget`
  (bind _result (`/Engine/EditorBlueprintResources/StandardMacros.IncrementInt` (`self.CurrentIndex`))
    (:`  `
      (set `self.CurrentIndex` _result)
      (if (>= (`self.CurrentIndex`) (`KismetArrayLibrary.Array_Length` (`self.GuidePoints`)))
        (set `self.FinalLocation` true)
        (else
          (bind _output_get (set `self.TargetLocation` (`self.K2_GetActorLocation` (`|GetArrayItem` (`self.GuidePoints`) (`self.CurrentIndex`)))))
          (`KismetSystemLibrary.PrintString` (`KismetStringLibrary.Conv_VectorToString` _output_get) true true (struct :`G` 0.66 :`B` 1.0 :`A` 1.0) 10.0))))))

(fn `ChangeToMoving`
  (if (and (< (`KismetMathLibrary.Vector_Distance` (`self.K2_GetActorLocation`) (`self.K2_GetActorLocation` (`GameplayStatics.GetPlayerPawn` 0))) 100.0) (< (`self.CurrentIndex`) (`KismetArrayLibrary.Array_Length` (`self.GuidePoints`))))
    (set `self.IsMoving` true)))

(fn `MoveToNextTarget`
  (`self.K2_SetActorLocation` (`KismetMathLibrary.VInterpTo_Constant` (`self.K2_GetActorLocation`) (`self.TargetLocation`) (`GameplayStatics.GetWorldDeltaSeconds`) (`self.Speed`))))

(fn `UserConstructionScript`)